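; Throwable closed-book prop Blueprint with a grab component and randomized appearance.
; On BeginPlay it picks one of three materials at random and applies a slight random scale per axis to its static mesh.
; Grabbing it sets BookFacts to a fixed question key, but the fact-text selection nodes are left unconnected, so no text is produced here.
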(event `self.ReceiveBeginPlay`
  (bind _returnvalue (`KismetMathLibrary.RandomFloatInRange` 1.0 1.3))
  (`PrimitiveComponent.SetMaterial` (`self.StaticMesh`) 0 (`|GetArrayItem` (`self.Materials`) (`KismetMathLibrary.RandomIntegerInRange` 0 2)))
  (`SceneComponent.SetWorldScale3D` (`self.StaticMesh`) (`KismetMathLibrary.MakeVector` _returnvalue _returnvalue _returnvalue)))

(event `self.GrabComponent.OnGrabbed`
  (bind _output_get (set `self.Book_Facts` "Question_1")))

(fn `UserConstructionScript`)