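; Planets question actor that shows the name of whichever solar system body the player grabs.
; Each body, from the Sun through Pluto, has its own grab component whose OnGrabbed event stores a hardcoded name in SelectedPlanet and writes it to SelectedText.
; No answer checking happens in this Blueprint; it only records and displays the latest selection.
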(event `self.MarsGrabComponent.OnGrabbed`
  (bind _output_get (set `self.Selected_Planet` "Mars"))
  (`TextRenderComponent.K2_SetText` (`self.Selected Text`) (`KismetTextLibrary.Conv_NameToText` _output_get)))

(event `self.EarthGrabComponent.OnGrabbed`
  (bind _output_get (set `self.Selected_Planet` "Earth"))
  (`TextRenderComponent.K2_SetText` (`self.Selected Text`) (`KismetTextLibrary.Conv_NameToText` _output_get)))

(event `self.SunGrabComponent.OnGrabbed`
  (bind _output_get (set `self.Selected_Planet` "Sun"))
  (`TextRenderComponent.K2_SetText` (`self.Selected Text`) (`KismetTextLibrary.Conv_NameToText` _output_get)))

(event `self.MercuryGrabComponent.OnGrabbed`
  (bind _output_get (set `self.Selected_Planet` "Mercury"))
  (`TextRenderComponent.K2_SetText` (`self.Selected Text`) (`KismetTextLibrary.Conv_NameToText` _output_get)))

(event `self.VenusGrabComponent.OnGrabbed`
  (bind _output_get (set `self.Selected_Planet` "Venus"))
  (`TextRenderComponent.K2_SetText` (`self.Selected Text`) (`KismetTextLibrary.Conv_NameToText` _output_get)))

(event `self.NeptuneGrabComponent.OnGrabbed`
  (bind _output_get (set `self.Selected_Planet` "Neptune"))
  (`TextRenderComponent.K2_SetText` (`self.Selected Text`) (`KismetTextLibrary.Conv_NameToText` _output_get)))

(event `self.PlutoGrabComponent.OnGrabbed`
  (bind _output_get (set `self.Selected_Planet` "Pluto"))
  (`TextRenderComponent.K2_SetText` (`self.Selected Text`) (`KismetTextLibrary.Conv_NameToText` _output_get)))

(event `self.JupiterGrabComponent.OnGrabbed`
  (bind _output_get (set `self.Selected_Planet` "Jupiter"))
  (`TextRenderComponent.K2_SetText` (`self.Selected Text`) (`KismetTextLibrary.Conv_NameToText` _output_get)))

(event `self.SaturnGrabComponent.OnGrabbed`
  (bind _output_get (set `self.Selected_Planet` "Saturn"))
  (`TextRenderComponent.K2_SetText` (`self.Selected Text`) (`KismetTextLibrary.Conv_NameToText` _output_get)))

(event `self.UranusGrabComponent.OnGrabbed`
  (bind _output_get (set `self.Selected_Planet` "Uranus"))
  (`TextRenderComponent.K2_SetText` (`self.Selected Text`) (`KismetTextLibrary.Conv_NameToText` _output_get)))

(fn `UserConstructionScript`)